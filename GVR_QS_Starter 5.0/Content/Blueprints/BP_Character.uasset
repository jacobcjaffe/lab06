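; BP_Character is a first-person-style player character with axis-driven movement, mouse look and a gaze check for interacting with whatever the camera faces.
; Every Tick, GazeCheck runs a Visibility line trace forward from the camera, with debug drawing on.
; On a hit it calls InteractMessage on the hit actor every frame without a button press; otherwise it prints a not-touching debug string.
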(event `InputAxis|moveLeft`
  (params (AxisValue :type "Float (single-precision)"))
  ;[1 1 1] Input
  (`self.AddMovementInput` (`self.GetActorRightVector`) AxisValue))

(event `self.ReceiveTick`
  (params (DeltaSeconds :type "Float (single-precision)"))
  (`self.GazeCheck`))

(event `InputAxis|mouseX`
  (params (AxisValue :type "Float (single-precision)"))
  ;[1 1 1] Input
  (`self.AddControllerYawInput` AxisValue))

(event `InputAxis|mouseY`
  (params (AxisValue :type "Float (single-precision)"))
  ;[1 1 1] Input
  (`self.AddControllerPitchInput` AxisValue))

(event `InputAxis|moveUp`
  (params (AxisValue :type "Float (single-precision)"))
  ;[1 1 1] Input
  (`self.AddMovementInput` (`self.GetActorForwardVector`) AxisValue))

(event `GazeCheck`
  (bind _camera (`self.Camera`))
  (bind _returnvalue (`SceneComponent.K2_GetComponentLocation` _camera))
  ;[1 1 1] Gaze check
  (bind (_outhit _returnvalue_2) (`KismetSystemLibrary.LineTraceSingle` :`Start` _returnvalue :`End` (+ _returnvalue (* (`SceneComponent.GetForwardVector` _camera) 2000)) :`TraceChannel` "TraceTypeQuery1" :`DrawDebugType` "ForOneFrame"))
  (if _returnvalue_2
    (message `/Game/Blueprints/BP_interact_interface.interact` (`.HitActor` (`GameplayStatics.BreakHitResult` _outhit)))
    (else
      (`KismetSystemLibrary.PrintString` "Not Touching" true true (struct :`G` 0.66 :`B` 1.0 :`A` 1.0) 2.0 "1"))))

(fn `UserConstructionScript`)